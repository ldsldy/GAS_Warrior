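; Base projectile Blueprint that handles the cosmetic sound and Niagara effects of a projectile's spawn, flight and impact.
; BeginPlay plays the spawn sound, attaches the fly sound to the root and spawns a forward-facing muzzle system, though no template is wired.
; The ProjectileImpact event plays the impact sound at the actor and spawns the impact effect with no location wired.
; Validity checks guard each asset variable; the graph holds no movement, collision or damage logic.
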(event `self.ReceiveBeginPlay`
  (`|ExecutionSequence`
    (:`then_0`
      (bind _projectilespawnsound (`self.ProjectileSpawnSound`)
        (:`then`
          (`GameplayStatics.PlaySoundAtLocation` _projectilespawnsound (`self.K2_GetActorLocation`) (struct) 1.0 1.0 0.0 null null null null))
        (:`else`)))
    (:`then_1`
      (bind _projectileflysound (`self.ProjectileFlySound`)
        (:`then`
          (`GameplayStatics.SpawnSoundAttached` _projectileflysound (`self.RootComponent`) "None" (0.0 0.0 0.0) (struct) "KeepRelativeOffset" true 1.0 1.0 0.0 null null))
        (:`else`)))
    (:`then_2`
      (`self.ProjectileMuzzleFX`
        (:`then`
          (`NiagaraFunctionLibrary.SpawnSystemAtLocation` null (`self.K2_GetActorLocation`) (`KismetMathLibrary.Conv_VectorToRotator` (`self.GetActorForwardVector`))))
        (:`else`)))))

(event `ProjectileImpact`
  (`|ExecutionSequence`
    (:`then_0`
      (bind _projectileimapctsound (`self.ProjectileImapctSound`)
        (:`then`
          (`GameplayStatics.PlaySoundAtLocation` _projectileimapctsound (`self.K2_GetActorLocation`) (struct) 1.0 1.0 0.0 null null null null))
        (:`else`)))
    (:`then_1`
      (bind _projectileimpatfx (`self.ProjectileImpatFX`)
        (:`then`
          (`NiagaraFunctionLibrary.SpawnSystemAtLocation` _projectileimpatfx))
        (:`else`)))))

(fn `UserConstructionScript`)