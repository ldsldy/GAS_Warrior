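; BP_EnemyCharacter_Base is an enemy character Blueprint that handles death with a dissolve effect.
; OnEnemyDied pauses mesh animation, disables capsule collision and plays DissolveTimeline at a rate scaled by TotalDissolveTime.
; The timeline's normalized track drives the DissolveAmount material parameter on the mesh.
; DestroyActor follows that parameter write on the Update path, so it runs on the first update rather than on Finished.
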(event `/Game/EnemyCharacter/BPI_EnemyDeath.OnEnemyDied`
  (`|ExecutionSequence`
    (:`then_0`
      (set `SkeletalMeshComponent.bPauseAnims` true (`self.Mesh`))
      (`PrimitiveComponent.SetCollisionEnabled` (`self.CapsuleComponent`) "NoCollision"))
    (:`then_1`
      (`TimelineComponent.SetPlayRate` (`self.DissolveTimeline`) (/ 1.0 (`self.TotalDissolveTime`)))
      (bind (_direction _normalizedfloattrack) (`Timeline|DissolveTimeline` :!via `PlayFromStart`)
        (:`Update`
          (`MeshComponent.SetScalarParameterValueOnMaterials` (`self.Mesh`) "DissolveAmount" _normalizedfloattrack)
          (`self.K2_DestroyActor`))))))

(fn `UserConstructionScript`)